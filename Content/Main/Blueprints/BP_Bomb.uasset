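; BP_Bomb is a bomb actor that explodes on impact and can hurt the player.
; When the Bomb component registers a hit, it spawns a scaled-up explosion emitter and sound at the impact point, then destroys the actor.
; It then measures the distance from the impact to player 0's BP_Player pawn, applying knockback away from the blast and fixed damage if within ExplosionRadius.
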(event OnComponentHit(Bomb)
  (params (HitComponent :type Primitive%20Component%20Object%20Reference) (OtherActor :type Actor%20Object%20Reference) (OtherComp :type Primitive%20Component%20Object%20Reference) (NormalImpulse :type Vector :default "0, 0, 0") (Hit :type Hit%20Result%20Structure%20%28by%20ref%29))
  (bind _location (Collision|BreakHitResult Hit))
  (Effects|SpawnEmitteratLocation "/Game/StarterContent/Particles/P_Explosion.P_Explosion" _location "0, 0, 0" "5.000000,5.000000,5.000000")
  (Audio|PlaySoundatLocation "/Game/StarterContent/Audio/Explosion01.Explosion01" _location "0, 0, 0" 1.0 1.0 0.0 0 0 0)
  (Actor|DestroyActor)
  (bind _asbp_player (Utilities|Casting|CastToBP_Player (Game|Player|GetPlayerPawn 0)))
  (if (<= (Math|Vector|Distance(Vector) (Transformation|GetActorLocation _asbp_player) _location) (Variables|Default|GetExplosionRadius))
    (Default|KnockBackPlayer _asbp_player _location 1e+03)
    (Default|TakeDamage _asbp_player 1e+01)))

(event EventBeginPlay)

(event Collision|EventActorBeginOverlap
  (params (OtherActor :type Actor%20Object%20Reference)))

(event EventTick
  (params (DeltaSeconds :type Float%20%28single-precision%29)))

(fn ConstructionScript)