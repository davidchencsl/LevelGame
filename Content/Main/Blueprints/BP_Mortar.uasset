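; BP_Mortar is a stationary enemy mortar that lobs bombs at the player within its firing sphere.
; A looping timer checks range and rolls a random fire chance, then spawns a BP_Bomb at the launch point.
; A suggested high-arc projectile velocity, aimed at the player with random scatter, sets the bomb's physics velocity.
; A BP_Player overlapping the Head component destroys the mortar.
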(event OnComponentBeginOverlap(Head)
  (params (OverlappedComponent :type Primitive%20Component%20Object%20Reference) (OtherActor :type Actor%20Object%20Reference) (OtherComp :type Primitive%20Component%20Object%20Reference) (OtherBodyIndex :type Integer) (bFromSweep :type Boolean) (SweepResult :type Hit%20Result%20Structure%20%28by%20ref%29))
  (Utilities|Casting|CastToBP_Player OtherActor)
  (Actor|DestroyActor))

(event Custom|Fire
  (bind _returnvalue (Game|GetPlayerCharacter 0))
  (bind _randomradius (Variables|Default|GetRandomRadius))
  (bind _randomradius_2 (Variables|Default|GetRandomRadius))
  (bind _fireradius (Variables|Default|GetFireRadius))
  (bind _returnvalue_2 (Transformation|GetActorLocation _returnvalue))
  (bind _returnvalue_3 (- 0.0 _randomradius))
  (bind _returnvalue_4 (Math|Random|RandomFloatinRange _returnvalue_3 _randomradius_2))
  (if (<= (Math|Vector|Distance(Vector) _returnvalue_2 (Transformation|GetWorldLocation _fireradius)) (Components|Sphere|GetScaledSphereRadius _fireradius))
    (if (< (Math|Random|RandomFloat) (Variables|Default|GetFireRate))
      (bind _returnvalue_5 (Game|SpawnActorfromClass "/Game/Main/Blueprints/BP_Bomb.BP_Bomb_C" (Math|Transform|MakeTransform (Transformation|GetWorldLocation (Variables|Default|GetLaunchPoint)) "0, 0, 0" "1,1,1") "AdjustIfPossibleButAlwaysSpawn" 0 0))
      (bind _tossvelocity (Class|GameplayStatics|BlueprintSuggestProjectileVelocity (Transformation|GetWorldLocation (Variables|/Game/Main/Blueprints/BP_Bomb.BP_Bomb_C|GetBomb _returnvalue_5)) (+ _returnvalue_2 (Math|Vector|MakeVector _returnvalue_4 _returnvalue_4 0.0)) (Variables|Default|GetLaunchSpeed) 0.0 "DoNotTrace" 1.0 true false))
      (Physics|SetPhysicsLinearVelocity (Variables|/Game/Main/Blueprints/BP_Bomb.BP_Bomb_C|GetBomb _returnvalue_5) _tossvelocity false "None"))))

(event EventBeginPlay
  (Utilities|Time|SetTimerbyEvent (delegate Custom|Fire) (Variables|Default|GetFireInterval) true))

(event Collision|EventActorBeginOverlap
  (params (OtherActor :type Actor%20Object%20Reference)))

(event EventTick
  (params (DeltaSeconds :type Float%20%28single-precision%29)))

(fn ConstructionScript)