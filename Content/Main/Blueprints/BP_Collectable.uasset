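; BP_Collectable is a pickup that spins and bobs in place until the player touches it.
; Sphere overlap with BP_Player increments the player's Collected count, refreshes its collectable text and destroys the pickup.
; Tick rotates the mesh on yaw by RotationSpeed scaled by delta time and adds a sine-based local Z offset from OscillateSpeed and Amplitude, not scaled by delta time.
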(event OnComponentBeginOverlap(Sphere)
  (params (OverlappedComponent :type Primitive%20Component%20Object%20Reference) (OtherActor :type Actor%20Object%20Reference) (OtherComp :type Primitive%20Component%20Object%20Reference) (OtherBodyIndex :type Integer) (bFromSweep :type Boolean) (SweepResult :type Hit%20Result%20Structure%20%28by%20ref%29))
  (bind _asbp_player (Utilities|Casting|CastToBP_Player OtherActor))
  (Math|Integer|IncrementInt (Variables|/Game/Main/Blueprints/BP_Player.BP_Player_C|GetCollected _asbp_player)
    (:%20%20
      (Default|UpdateCollectableText _asbp_player)
      (Actor|DestroyActor))))

(event EventBeginPlay)

(event EventTick
  (params (DeltaSeconds :type Float%20%28single-precision%29))
  ;[1 1 1] Local Movement
  (Transformation|AddLocalRotation (Variables|Default|GetSM_Collectible_Common) (Math|Rotator|MakeRotator 0.0 0.0 (* (Variables|Default|GetRotationSpeed) DeltaSeconds)) false false)
  (Transformation|AddLocalOffset (Variables|Default|GetSM_Collectible_Common) (Math|Vector|MakeVector 0.0 0.0 (* (Math|Trig|Sin(Radians) (* (Actor|GetGameTimeSinceCreation) (Variables|Default|GetOscillateSpeed))) (Variables|Default|GetAmplitude))) false false))

(fn ConstructionScript)